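; NPC AI controller that runs a guard behavior tree on a patrol blackboard.
; On BeginPlay it initializes the blackboard, starts the tree and caches the blackboard component.
; AI Perception updates write any sensed actor lacking the "Enemy" tag to the enemy key, and clear that key when such an actor's stimulus is no longer sensed.
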(event `self.ReceiveBeginPlay`
  (bind _blackboardcomponent (`self.UseBlackboard` "/Game/Dynamic/NPC/AI/Blueprints/PatrolData.PatrolData"))
  (`self.RunBehaviorTree` "/Game/Dynamic/NPC/AI/Blueprints/GuardBehaviour.GuardBehaviour")
  (set `self.BlackBoardRef` _blackboardcomponent))

(event `self.AIPerception.OnTargetPerceptionUpdated`
  (params (Actor :type "Actor Object Reference") (Stimulus :type "AIStimulus Structure"))
  (bind _enemykey (`self.EnemyKey`))
  (bind _blackboardref (`self.BlackBoardRef`))
  (if (`self.ActorHasTag` Actor "Enemy")
    _
    (elif (`.bSuccessfullySensed` (break `AIStimulus` Stimulus))
      (`BlackboardComponent.SetValueAsObject` _blackboardref _enemykey Actor)
      (else
        (`BlackboardComponent.ClearValue` _blackboardref _enemykey)))))

(fn `UserConstructionScript`)