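; Terrain tile for an infinite-terrain game, driven by three player-only overlap events.
; Entering LockingVolume opens the Barrier and calls PlaceActors to scatter rocks, trees and street props.
; Leaving it closes the Barrier and asks InfinteTerrainGameMode to spawn another tile, while entering DestroyVolume destroys this one.
; GetAttachLocation exposes the Arrow's world transform as an attach point.
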(event `self.LockingVolume.OnComponentBeginOverlap`
  (params (OverlappedComponent :type "PrimitiveComponent Object Reference") (OtherActor :type "Actor Object Reference") (OtherComp :type "PrimitiveComponent Object Reference") (OtherBodyIndex :type Integer) (bFromSweep :type Boolean) (SweepResult :type "HitResult Structure (by ref)"))
  (`self.IsPlayerActor` OtherActor)
  (`self.UnlockLevel`)
  (`self.PlaceActors` "/Game/Dynamic/Terrain/Props/BP_Rock.BP_Rock_C" 1 10 400.0 0.5 5.0)
  (`self.PlaceActors` "/Game/Dynamic/Terrain/Props/BP_Tree_01.BP_Tree_01_C" 1 5 100.0 0.7 2.5)
  (`self.PlaceActors` "/Game/Dynamic/Terrain/Props/BP_Tree_02.BP_Tree_02_C" 1 5 100.0 0.7 2.5)
  (`self.PlaceActors` "/Game/Dynamic/Terrain/Props/BP_ParkBench.BP_ParkBench_C" 1 4 200.0)
  (`self.PlaceActors` "/Game/Dynamic/Terrain/Props/BP_Bin_01.BP_Bin_01_C" 1 2 100.0)
  (`self.PlaceActors` "/Game/Dynamic/Terrain/Props/BP_Bin_02.BP_Bin_02_C" 1 3 50.0)
  (`self.PlaceActors` "/Game/Dynamic/Terrain/Props/BP_Van.BP_Van_C" 1 3 300.0)
  (`self.PlaceActors` "/Game/Dynamic/Terrain/Props/BP_Newspapers.BP_Newspapers_C" 1 4 100.0))

(event `self.LockingVolume.OnComponentEndOverlap`
  (params (OverlappedComponent :type "PrimitiveComponent Object Reference") (OtherActor :type "Actor Object Reference") (OtherComp :type "PrimitiveComponent Object Reference") (OtherBodyIndex :type Integer))
  (`self.IsPlayerActor` OtherActor)
  (`self.LockLevel`)
  (bind _asinfinte_terrain_game_mode (cast `/Game/Dynamic/InfinteTerrainGameMode` (`GameplayStatics.GetGameMode`)))
  (`/Game/Dynamic/InfinteTerrainGameMode.SpawnTile` _asinfinte_terrain_game_mode))

(event `self.DestroyVolume.OnComponentBeginOverlap`
  (params (OverlappedComponent :type "PrimitiveComponent Object Reference") (OtherActor :type "Actor Object Reference") (OtherComp :type "PrimitiveComponent Object Reference") (OtherBodyIndex :type Integer) (bFromSweep :type Boolean) (SweepResult :type "HitResult Structure (by ref)"))
  (`self.IsPlayerActor` OtherActor)
  (`self.K2_DestroyActor`))

(fn `Get Attach Location`
  (returns (`Attach Transform` :type "Transform Structure"))
  (return (`SceneComponent.K2_GetComponentToWorld` (`self.Arrow`))))

(fn `LockLevel`
  (`PrimitiveComponent.SetCollisionEnabled` (`self.Barrier`) "QueryAndPhysics")
  (`PrimitiveComponent.SetMaterial` (`self.Barrier`) 0 "/Game/Dynamic/Terrain/Mi_Barrier_Closed.Mi_Barrier_Closed"))

(fn `UnlockLevel`
  (`PrimitiveComponent.SetCollisionEnabled` (`self.Barrier`) "NoCollision")
  (`PrimitiveComponent.SetMaterial` (`self.Barrier`) 0 "/Game/Dynamic/Terrain/Mi_Barrier_Open.Mi_Barrier_Open"))

(fn `UserConstructionScript`)