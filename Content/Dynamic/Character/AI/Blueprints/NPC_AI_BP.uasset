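; NPC AI controller that runs the guard behavior tree and feeds it targets from AI perception.
; On BeginPlay it sets up the patrol blackboard, starts the tree and caches the blackboard component.
; Perception updates for actors without the "Enemy" tag set the blackboard's enemy key when sensed and clear it when sensing is lost.
; Actors tagged "Enemy" are ignored.
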(event `self.ReceiveBeginPlay`
  (bind _blackboardcomponent (`self.UseBlackboard` "/Game/Dynamic/Character/AI/Blueprints/PatrolData.PatrolData"))
  (`self.RunBehaviorTree` "/Game/Dynamic/Character/AI/Blueprints/GuardBehaviour.GuardBehaviour")
  (set `self.BlackBoardRef` _blackboardcomponent))

(event `self.AIPerception.OnTargetPerceptionUpdated`
  (params (Actor :type "Actor Object Reference") (Stimulus :type "AIStimulus Structure"))
  (`self.UpdateBlackboardEnemyKey` Actor Stimulus))

(fn `UpdateBlackboardEnemyKey`
  (params (ObjectValue :type "Actor Object Reference") (AIStimulus :type "AIStimulus Structure (by ref)"))
  (bind _enemykey (`self.EnemyKey`))
  (bind _blackboardref (`self.BlackBoardRef`))
  (if (`self.ActorHasTag` ObjectValue "Enemy")
    _
    (elif (`.bSuccessfullySensed` (break `AIStimulus` AIStimulus))
      (`BlackboardComponent.SetValueAsObject` _blackboardref _enemykey ObjectValue)
      (else
        (`BlackboardComponent.ClearValue` _blackboardref _enemykey)))))

(fn `UserConstructionScript`)